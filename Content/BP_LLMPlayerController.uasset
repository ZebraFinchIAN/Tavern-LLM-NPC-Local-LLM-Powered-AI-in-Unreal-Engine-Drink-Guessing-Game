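; Player controller for an LLM-driven NPC dialogue game with a drink-guessing step, opening with an instructions widget.
; Pressing E line-traces forward from the pawn, binds to the hit AI character's conversation-update event, opens dialogue UI and starts it via AniyiBaslat.
; Each update rebuilds the scroll box from the NPC's conversation history.
; TahminiKontrolEt checks the chosen drink against the customer's DataTable row, sends the NPC the matching result prompt and reopens dialogue.
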(event Custom|OnKonusmaGuncellendi_Olay
  (Widget|Panel|ClearChildren (Variables|/Game/WBP_DialogueUI.WBP_DialogueUI_C|GetDialogueScrollBox (Variables|Default|GetDialogueUI_Reference)))
  (for _array_element (Variables|/Script/LLMProjem.AICharacter|GetKonusmaGecmisi (Variables|Default|GetCurrentNPC_Reference))
    (bind _returnvalue (UserInterface|CreateWidget "/Game/WBP_DialogueLine.WBP_DialogueLine_C"))
    (Default|SetDialogueData _returnvalue (.Speaker (Utilities|Struct|BreakConversationLine _array_element)) (.Line (Utilities|Struct|BreakConversationLine _array_element)))
    (Widget|Panel|AddChild (Variables|/Game/WBP_DialogueUI.WBP_DialogueUI_C|GetDialogueScrollBox (Variables|Default|GetDialogueUI_Reference)) _returnvalue))
  (Class|ScrollBox|ScrolltoEnd (Variables|/Game/WBP_DialogueUI.WBP_DialogueUI_C|GetDialogueScrollBox (Variables|Default|GetDialogueUI_Reference))))

(event EventBeginPlay
  (bind _returnvalue (UserInterface|CreateWidget "/Game/WBP_Instructions.WBP_Instructions_C"))
  (UserInterface|Viewport|AddtoViewport _returnvalue 0)
  (Input|SetInputModeUIOnly (Game|GetPlayerController 0) _returnvalue "DoNotLock" false)
  (Variables|Default|SetbShowMouseCursor true))

(event EventTick
  (params (DeltaSeconds :type Float%20%28single-precision%29)))

(event Input|KeyboardEvents|E
  (params (Key :type Key%20Structure :default "None"))
  (bind _returnvalue (Pawn|GetControlledPawn))
  (bind _returnvalue_2 (Transformation|GetActorLocation _returnvalue))
  (:Pressed
    (bind (_outhit _returnvalue_3) (Collision|LineTraceByChannel _returnvalue_2 (+ _returnvalue_2 (* (Transformation|GetActorForwardVector _returnvalue) 1.5e+03)) "TraceTypeQuery1" false 0 "ForDuration"))
    (if _returnvalue_3
      (bind _asbp_aicharacter_base (Utilities|Casting|CastToBP_AICharacter_Base (.HitActor (Collision|BreakHitResult _outhit)))
        (:then
          (Variables|Default|SetCurrentNPC_Reference _asbp_aicharacter_base)
          (EventDispatchers|AssignOnKonusmaGuncellendi (Variables|Default|GetCurrentNPC_Reference) (delegate Custom|OnKonusmaGuncellendi_Olay))
          (bind _returnvalue_4 (UserInterface|CreateWidget "/Game/WBP_DialogueUI.WBP_DialogueUI_C"))
          (bind _output_get (Variables|Default|SetDialogueUI_Reference _returnvalue_4))
          (UserInterface|Viewport|AddtoViewport _output_get 0)
          (Input|SetInputModeGameandUI self (Variables|Default|GetDialogueUI_Reference) "DoNotLock" true false)
          (Variables|Default|SetbShowMouseCursor true)
          (Class|AICharacter|AniyiBaslat (Variables|Default|GetCurrentNPC_Reference)))
        (:CastFailed
          (Development|PrintString "AI Character Değil"))))))

(fn ConstructionScript)

(fn TahminiKontrolEt
  (params (SecilenIcecekID :type Name))
  (bind _currentnpc_reference (Variables|Default|GetCurrentNPC_Reference))
  (bind _currentnpc_reference_2 (Variables|Default|GetCurrentNPC_Reference))
  (bind _returnvalue (Utilities|GetDataTableRow (Variables|/Script/LLMProjem.AICharacter|GetMusteriVeriTablosu _currentnpc_reference) (Variables|/Script/LLMProjem.AICharacter|GetAktifMusteriKimligi _currentnpc_reference))
    (:then
      (if true
        (if (== SecilenIcecekID (.Dogru_Icecek_Kimligi (Utilities|Struct|BreakST_MusteriAnisi _returnvalue)))
          (Variables|/Script/LLMProjem.AICharacter|SetKonusmaAsamasi _currentnpc_reference_2 2)
          (Class|AICharacter|TahminSonucunuBildir _currentnpc_reference_2 (.Dogru_Secim_Promptu (Utilities|Struct|BreakST_MusteriAnisi _returnvalue)))
          (else
            (Class|AICharacter|TahminSonucunuBildir (Variables|Default|GetCurrentNPC_Reference) (.Yanlis_Secim_Promptu (Utilities|Struct|BreakST_MusteriAnisi _returnvalue)))))
        (Widget|RemovefromParent (Variables|Default|GetGuessMenu_Reference))
        (bind _returnvalue_2 (UserInterface|CreateWidget "/Game/WBP_DialogueUI.WBP_DialogueUI_C"))
        (Variables|Default|SetDialogueUI_Reference _returnvalue_2)
        (UserInterface|Viewport|AddtoViewport (Variables|Default|GetDialogueUI_Reference) 0)
        (Input|SetInputModeGameandUI self (Variables|Default|GetDialogueUI_Reference) "DoNotLock" true false)
        (Variables|/Script/Engine.PlayerController|SetbShowMouseCursor (Game|GetPlayerController 0) true)))))